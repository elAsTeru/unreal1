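; Anim notify state that marks the window in an attack animation during which the character accepts combo input.
; On begin it casts the mesh owner to ThirdPersonCharacter and sets AcceptAttack to true, and on end it sets it back to false.
; Both events call the parent implementation first and return its result.
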(fn `Received_NotifyBegin`
  (params (MeshComp :type "SkeletalMeshComponent Object Reference") (Animation :type "AnimSequenceBase Object Reference") (TotalDuration :type "Float (double-precision)"))
  (returns (ReturnValue :type Boolean))
  (bind _returnvalue (`parent.Received_NotifyBegin` MeshComp Animation TotalDuration))
  (bind _asthird_person_character (cast `/Game/DragonGirl/BP/ThirdPersonCharacter` (`ActorComponent.GetOwner` MeshComp))
    (:`then`
      (set `/Game/DragonGirl/BP/ThirdPersonCharacter.AcceptAttack` true _asthird_person_character))
    (:`CastFailed`
      _))
  (return _returnvalue))

(fn `Received_NotifyEnd`
  (params (MeshComp :type "SkeletalMeshComponent Object Reference") (Animation :type "AnimSequenceBase Object Reference"))
  (returns (ReturnValue :type Boolean))
  (bind _returnvalue (`parent.Received_NotifyEnd` MeshComp Animation))
  (bind _asthird_person_character (cast `/Game/DragonGirl/BP/ThirdPersonCharacter` (`ActorComponent.GetOwner` MeshComp))
    (:`then`
      (set `/Game/DragonGirl/BP/ThirdPersonCharacter.AcceptAttack` false _asthird_person_character))
    (:`CastFailed`
      _))
  (return _returnvalue))